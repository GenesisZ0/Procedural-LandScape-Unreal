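; BP_MapGeneration is an actor that builds a procedural terrain mesh with collision at BeginPlay.
; CreateVertice fills a scaled grid of vertices and UVs, setting height from two multiplied 1D Perlin samples rather than true 2D noise.
; CreateTriangles indexes two triangles per cell, then CreateLandscape builds the mesh section and applies the material.
; DestroyLandScape clears the mesh, but neither it nor GenratePerlinNoise2d is called here.
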(event `self.ReceiveBeginPlay`
  (`self.CreateLandscape`))

(fn `CreateLandscape`
  (`self.CreateVertice`)
  (`self.CreateTriangles`)
  (`ProceduralMeshComponent.CreateMeshSection_LinearColor` :`self` (`self.ProceduralMesh`) :`Vertices` (`self.Vertices`) :`Triangles` (`self.Triangles`) :`UV0` (`self.UV0`) :`bCreateCollision` true)
  (`PrimitiveComponent.SetMaterial` (`self.ProceduralMesh`) 0 (`self.Material`)))

(fn `CreateTriangles`
  (locals (Vertex :type Integer))
  (for _ (range (`self.Xsize`))
    (for _ (range (`self.Ysize`))
      (`KismetArrayLibrary.Array_Add` (`self.Triangles`) (`local.Vertex`))
      (`KismetArrayLibrary.Array_Add` (`self.Triangles`) (+ (`local.Vertex`) 1))
      (`KismetArrayLibrary.Array_Add` (`self.Triangles`) (+ (`self.Ysize`) (`local.Vertex`) 1))
      (`KismetArrayLibrary.Array_Add` (`self.Triangles`) (+ (`local.Vertex`) 1))
      (`KismetArrayLibrary.Array_Add` (`self.Triangles`) (+ (`self.Ysize`) (`local.Vertex`) 2))
      (`KismetArrayLibrary.Array_Add` (`self.Triangles`) (+ (`self.Ysize`) (`local.Vertex`) 1))
      (`/Engine/EditorBlueprintResources/StandardMacros.IncrementInt` (`local.Vertex`)))
    (`/Engine/EditorBlueprintResources/StandardMacros.IncrementInt` (`local.Vertex`))))

(fn `CreateVertice`
  (locals (X :type Integer) (Y :type Integer))
  (for _index (range (+ (`self.Xsize`) 1))
    (set `local.X` _index)
    (for _index_2 (range (+ (`self.Ysize`) 1))
      (set `local.Y` _index_2)
      (`KismetArrayLibrary.Array_Add` (`self.Vertices`) (`KismetMathLibrary.MakeVector` (* (`local.X`) (`self.Scale`)) (* (`local.Y`) (`self.Scale`)) (* (* (`KismetMathLibrary.PerlinNoise1D` (+ (`KismetMathLibrary.Conv_IntToDouble` (`local.X`)) 0.1)) (`KismetMathLibrary.PerlinNoise1D` (+ (`KismetMathLibrary.Conv_IntToDouble` (`local.Y`)) 0.1))) (`self.ZMultiplier`))))
      (`KismetArrayLibrary.Array_Add` (`self.UV0`) (`KismetMathLibrary.MakeVector2D` (* (`local.X`) (`self.UvScale`)) (* (`local.Y`) (`self.UvScale`)))))))

(fn `DestroyLandScape`
  (`ProceduralMeshComponent.ClearMeshSection` (`self.ProceduralMesh`) 0)
  (`ProceduralMeshComponent.ClearAllMeshSections` (`self.ProceduralMesh`))
  (`ProceduralMeshComponent.ClearAllMeshSections` (`self.ProceduralMesh`)))

(fn `GenratePerlinNoise2d`
  (returns (Float :type "Float (double-precision)"))
  (locals (Time :type "Float (double-precision)"))
  (for _index (range (+ (`self.Xsize`) 1))
    (`/Engine/EditorBlueprintResources/StandardMacros.IncrementFloat` (`local.Time`)
      (:`  `
        (return (`KismetMathLibrary.PerlinNoise1D` (`KismetMathLibrary.Conv_IntToDouble` _index)))))))

(fn `UserConstructionScript`)